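; Player character Blueprint with walk, look, jump and sprint input, plus weapon pickup, drop and shooting.
; AddToInterract stores a candidate weapon; Activate drops any held weapon and attaches it to WeaponPlac, toggling mesh physics on pickup and drop.
; Shooting checks and spends the character's WeaponAmmo, playing a sound when empty.
; Damage feeds BioStat; zero HP triggers ragdoll and notifies MainController, while Tick prints HP and ammo.
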(event EventBeginPlay
  ;[1 1 1] В начале
)

(event Collision|EventActorBeginOverlap
  (params (OtherActor :type Actor%20Object%20Reference)))

(event EventTick
  (params (DeltaSeconds :type Float%20%28single-precision%29))
  (Development|PrintString (Utilities|String|Append "HP:" (Utilities|String|ToString(Float) (Variables|/Game/GBAlexandr/BluePrints/Characters/BioStat.BioStat_C|GetCurrentHP (Variables|Default|GetBioStat))) " AMMO:" (Utilities|String|ToString(Integer) (Variables|/Game/GBAlexandr/BluePrints/Characters/WeaponAmmo.WeaponAmmo_C|GetCurrentAmmo (Variables|Default|GetWeaponAmmo)))) true true "(R=0.000000,G=0.660000,B=1.000000,A=1.000000)" (Utilities|Time|GetWorldDeltaSeconds)))

(event Game|Damage|EventAnyDamage
  (params (Damage :type Float%20%28single-precision%29) (DamageType :type Damage%20Type%20Object%20Reference) (InstigatedBy :type Controller%20Object%20Reference) (DamageCauser :type Actor%20Object%20Reference))
  (Default|MakeDamage (Variables|Default|GetBioStat) Damage)
  (if (<= (Variables|/Game/GBAlexandr/BluePrints/Characters/BioStat.BioStat_C|GetCurrentHP (Variables|Default|GetBioStat)) 0.0)
    (Physics|SetSimulatePhysics (Variables|Character|GetMesh) true)
    (bind _asmain_controller (Utilities|Casting|CastToMainController (Pawn|GetController)))
    (Default|Dead _asmain_controller)))

(event Input|ActionEvents|InputActionActivate
  (params (Key :type Key%20Structure :default "None"))
  ;[1 1 1] Входные данные Action
  (:Pressed
    (CallFunction|TakeWapon)))

(event Input|ActionEvents|InputActionSprint
  (params (Key :type Key%20Structure :default "None"))
  (bind _charactermovement (Variables|Character|GetCharacterMovement))
  ;[1 1 1] Входные данные Axis
  (:Pressed
    (Variables|/Script/Engine.CharacterMovementComponent|SetMaxWalkSpeed _charactermovement 1e+03))
  (:Released
    (Variables|/Script/Engine.CharacterMovementComponent|SetMaxWalkSpeed _charactermovement 6e+02)))

(event Input|ActionEvents|InputActionJump
  (params (Key :type Key%20Structure :default "None"))
  ;[1 1 1] Входные данные Axis
  (:Pressed
    (Character|Jump)))

(event Input|ActionEvents|InputActionDrop
  (params (Key :type Key%20Structure :default "None"))
  ;[1 1 1] Выбрасывание объекта
  (:Pressed
    (CallFunction|DropWeapon)))

(event Input|ActionEvents|InputActionShoot
  (params (Key :type Key%20Structure :default "None"))
  ;[1 1 1] Провера на оружие
  (:Pressed
    (if (Utilities|IsValid (Variables|Default|GetActiveWeapon))
      ;[1 1 1] Проверка патронов
      (bind _result (Default|CheckAmmo (Variables|Default|GetWeaponAmmo) 1))
      (if _result
        (Default|StartShoot (Variables|Default|GetActiveWeapon))
        (Default|SubtractAmmo (Variables|Default|GetWeaponAmmo) 1)
        (else
          (Audio|PlaySoundatLocation "/Engine/EditorSounds/Notifications/CompileFailed_Cue.CompileFailed_Cue" (Transformation|GetActorLocation) "0, 0, 0" 1.0 1.0 0.0 0 0 0))))))

(event Input|AxisEvents|InputAxisMoveForward
  (params (AxisValue :type Float%20%28single-precision%29))
  ;[1 1 1] Входные данные Axis
  (Pawn|Input|AddMovementInput (Transformation|GetActorForwardVector) AxisValue false))

(event Input|AxisEvents|InputAxisMoveRight
  (params (AxisValue :type Float%20%28single-precision%29))
  ;[1 1 1] Входные данные Axis
  (Pawn|Input|AddMovementInput (Transformation|GetActorRightVector) AxisValue false))

(event Input|AxisEvents|InputAxisLookUp
  (params (AxisValue :type Float%20%28single-precision%29))
  ;[1 1 1] Входные данные Axis
  (Pawn|Input|AddControllerPitchInput AxisValue))

(event Input|AxisEvents|InputAxisTurn
  (params (AxisValue :type Float%20%28single-precision%29))
  ;[1 1 1] Входные данные Axis
  (Pawn|Input|AddControllerYawInput AxisValue))

(fn ConstructionScript)

(fn AddtoInterract
  (params (Weapon :type Weapon%20Object%20Reference))
  (Variables|Default|SetInterractWeapon Weapon))

(fn TakeWapon
  (bind _interractweapon (Variables|Default|GetInterractWeapon))
  (Development|PrintString (Utilities|GetDisplayName _interractweapon))
  ;[1 1 1] Проверка валидности переменной
  (if (Utilities|IsValid _interractweapon)
    (if (Utilities|IsValid (Variables|Default|GetActiveWeapon))
      (CallFunction|DropWeapon))
    ;[1 1 1] Прикрепляет объект к компоненту
    (Transformation|AttachComponentToComponent (Variables|Default|GetInterractWeapon) (Variables|Default|GetWeaponPlac) "None" "SnapToTarget" "SnapToTarget" "KeepRelative" true)
    ;[1 1 1] Отключиние физики оружия
    (Physics|SetSimulatePhysics (Variables|/Game/GBAlexandr/BluePrints/Weapons/Weapon.Weapon_C|GetSkeletalMesh (Variables|Default|GetInterractWeapon)) false)
    (Variables|Default|SetActiveWeapon (Variables|Default|GetInterractWeapon))))

(fn DropWeapon
  ;[1 1 1] Открепляем объект
  (Transformation|DetachFromActor (Variables|Default|GetActiveWeapon) "KeepWorld" "KeepWorld" "KeepWorld")
  ;[1 1 1] Включаем физику
  (Physics|SetSimulatePhysics (Variables|/Game/GBAlexandr/BluePrints/Weapons/Weapon.Weapon_C|GetSkeletalMesh (Variables|Default|GetActiveWeapon)) true)
  (Variables|Default|SetActiveWeapon 0))