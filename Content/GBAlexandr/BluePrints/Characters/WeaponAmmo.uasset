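; WeaponAmmo tracks a current ammo count against a maximum for weapon use.
; On BeginPlay it sets the current count to a tenth of the maximum, truncated to an integer.
; SubtractAmmo reduces the count by a given amount, clamped between zero and the maximum, and CheckAmmo reports whether enough remains for a requested amount.
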(event EventBeginPlay
  (Variables|Default|SetCurrentAmmo (Math|Float|Truncate (* (Variables|Default|GetMaxAmmo) 0.1))))

(event EventTick
  (params (DeltaSeconds :type Float%20%28single-precision%29)))

(fn SubtractAmmo
  (params (Ammo :type Integer))
  (Variables|Default|SetCurrentAmmo (Math|Integer|Clamp(Integer) (- (Variables|Default|GetCurrentAmmo) Ammo) 0 (Variables|Default|GetMaxAmmo))))

(fn CheckAmmo
  (params (Ammo :type Integer))
  (return (>= (Variables|Default|GetCurrentAmmo) Ammo)))