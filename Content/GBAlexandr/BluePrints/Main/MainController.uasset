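; MainController is the player controller that owns the main HUD and keeps it in sync with the controlled MainCharacter.
; BeginPlay creates the MainGUI widget, adds it to the viewport and caches the pawn cast to MainCharacter.
; Tick polls the character to push health ratio, the name of the interactable weapon and active weapon ammo, hiding readouts without a valid weapon.
; The Dead event plays the GUI's game over screen.
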(event Custom|Dead
  (Default|PlayGameOverScreen (Variables|Default|Get%20MainGUI)))

(event EventBeginPlay
  ;[1 1 1] Создаем виджет и записываем ссылку на него
  (bind _returnvalue (UserInterface|CreateWidget "/Game/GBAlexandr/GUI/MainGUI.MainGUI_C"))
  (Variables|Default|Set%20MainGUI _returnvalue)
  ;[1 1 1] Добовляем виджет на экран
  (UserInterface|Viewport|AddtoViewport (Variables|Default|Get%20MainGUI) 0)
  ;[1 1 1] Уточняем класс управляемого персонажа
  (bind _asmain_character (Utilities|Casting|CastToMainCharacter (Pawn|GetControlledPawn))
    (:then
      ;[1 1 1] Записываем ссылку на персонажа типа MainCharacter
      (Variables|Default|SetMainChar _asmain_character))
    (:CastFailed
      (Development|PrintString "Cast failed"))))

(event EventTick
  (params (DeltaSeconds :type Float%20%28single-precision%29))
  (bind __maingui (Variables|Default|Get%20MainGUI))
  (bind _mainchar (Variables|Default|GetMainChar))
  (bind __maingui_2 (Variables|Default|Get%20MainGUI))
  (bind _weaponammo (Variables|/Game/GBAlexandr/BluePrints/Characters/MainCharacter.MainCharacter_C|GetWeaponAmmo _mainchar))
  (bind _activeweapon (Variables|/Game/GBAlexandr/BluePrints/Characters/MainCharacter.MainCharacter_C|GetActiveWeapon _mainchar))
  (bind _textammoinfo (Variables|/Game/GBAlexandr/GUI/MainGUI.MainGUI_C|GetTextAmmoInfo __maingui_2))
  (bind _biostat (Variables|/Game/GBAlexandr/BluePrints/Characters/MainCharacter.MainCharacter_C|GetBioStat _mainchar))
  (bind _interractweapon (Variables|/Game/GBAlexandr/BluePrints/Characters/MainCharacter.MainCharacter_C|GetInterractWeapon _mainchar))
  (Default|SetHP (Variables|Default|Get%20MainGUI) (/ (Variables|/Game/GBAlexandr/BluePrints/Characters/BioStat.BioStat_C|GetCurrentHP _biostat) (Variables|/Game/GBAlexandr/BluePrints/Characters/BioStat.BioStat_C|GetMaxHP _biostat)))
  (Utilities|FlowControl|Sequence
    (:then_0
      (if (Utilities|IsValid _interractweapon)
        (Default|SetInterractInfo __maingui "Visible" (Utilities|Text|ToText(String) (Utilities|GetDisplayName _interractweapon)))
        (else
          (Default|SetInterractInfo __maingui "Hidden"))))
    (:then_1
      (if (Utilities|IsValid _activeweapon)
        (Utilities|FlowControl|Sequence
          (:then_0
            (if (Utilities|IsValid (Variables|/Game/GBAlexandr/BluePrints/Characters/MainCharacter.MainCharacter_C|GetWeaponAmmo _mainchar))
              (Rendering|Components|TextRender|SetText _textammoinfo (Utilities|Text|ToText(String) (Utilities|String|Append (Utilities|String|ToString(Integer) (Variables|/Game/GBAlexandr/BluePrints/Characters/WeaponAmmo.WeaponAmmo_C|GetCurrentAmmo _weaponammo)) "/" (Utilities|String|ToString(Integer) (Variables|/Game/GBAlexandr/BluePrints/Characters/WeaponAmmo.WeaponAmmo_C|GetMaxAmmo _weaponammo))))))))))
    (:then_2
      (Widget|SetVisibility _textammoinfo (select (Utilities|IsValid _activeweapon) "Visible" "Hidden")))))

(fn ConstructionScript)